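; Basicitem is a pickup that adds its Worth to the Currency of Player1_BP.
; Overlap begin tells the player to show a pickup prompt, and overlap end removes the prompt and clears IsOverlappingItem.
; Tick polls IsPickedUp, which is not set in this graph, then credits player zero and destroys the item.
; The PickedUp event is an empty stub.
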(event Custom|PickedUp)

(event EventBeginPlay)

(event Collision|EventActorBeginOverlap
  (params (OtherActor :type Actor%20Object%20Reference))
  (bind _asplayer_1_bp (Utilities|Casting|CastToPlayer1_BP OtherActor))
  (Default|PickupPrompt _asplayer_1_bp))

(event EventTick
  (params (DeltaSeconds :type Float%20%28single-precision%29))
  (if (Variables|Default|GetIsPickedUp)
    (bind _asplayer_1_bp (Utilities|Casting|CastToPlayer1_BP (Game|GetPlayerCharacter 0))
      (:then
        (Variables|/Game/Blueprints/Player1_BP.Player1_BP_C|SetCurrency _asplayer_1_bp (+ (Variables|/Game/Blueprints/Player1_BP.Player1_BP_C|GetCurrency _asplayer_1_bp) (Variables|Default|GetWorth)))
        (Actor|DestroyActor))
      (:CastFailed
        (Development|PrintString "Cast To Player1BP  Failed (BasicItem)")))))

(event Collision|EventActorEndOverlap
  (params (OtherActor :type Actor%20Object%20Reference))
  (bind _asplayer_1_bp (Utilities|Casting|CastToPlayer1_BP OtherActor))
  (Default|PickupPromptDestroy (Variables|/Game/Blueprints/Player1_BP.Player1_BP_C|GetPickUpPromptRef _asplayer_1_bp))
  (Variables|/Game/Blueprints/Player1_BP.Player1_BP_C|SetIsOverlappingItem _asplayer_1_bp false))

(fn ConstructionScript)