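; Enemy actor that tracks health and reacts once when it runs out.
; AnyDamage subtracts the damage from Health and prints the new value.
; Tick polls Health and, through a DoOnce at zero or below, toggles visibility on StaticMesh and EnemyShapeTestDM and enables physics simulation on EnemyShapeTestDM, swapping the meshes on death.
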(event EventBeginPlay)

(event Collision|EventActorBeginOverlap
  (params (OtherActor :type Actor%20Object%20Reference)))

(event EventTick
  (params (DeltaSeconds :type Float%20%28single-precision%29))
  (if (<= (Variables|Default|GetHealth) 0.0)
    (Utilities|FlowControl|DoOnce false
      (:Completed
        (Rendering|ToggleVisibility (Variables|Default|GetEnemyShapeTest_DM) false)
        (Rendering|ToggleVisibility (Variables|Default|GetStaticMesh) false)
        (Physics|SetSimulatePhysics (Variables|Default|GetEnemyShapeTest_DM) true)))))

(event Game|Damage|EventAnyDamage
  (params (Damage :type Float%20%28single-precision%29) (DamageType :type Damage%20Type%20Object%20Reference) (InstigatedBy :type Controller%20Object%20Reference) (DamageCauser :type Actor%20Object%20Reference))
  (Variables|Default|SetHealth (- (Variables|Default|GetHealth) Damage))
  (Development|PrintString (Utilities|String|ToString(Float) (Variables|Default|GetHealth))))

(fn ConstructionScript)