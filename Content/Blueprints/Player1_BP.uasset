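; Player character Blueprint handling camera-relative movement, jump or item pickup, weapon index cycling, HUD and a pause menu widget.
; Holding fire builds Heat on Tick with a charge effect; release spawns an EnergyBlast only at low charge.
; Aiming makes the character follow controller yaw; the camera blend timeline is unconnected.
; Currency loads from a save slot on BeginPlay; Tick checks for death, then saves it and reopens the level.
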(event Custom|PauseMenuEvent
  (params (NewParam :type Boolean)))

(event Custom|Respawn
  (Game|OpenLevel(byName) "DefaultLevel"))

(event Custom|PickupPrompt
  ;[1 1 1] Pick Up Prompt
  (bind _returnvalue (UserInterface|CreateWidget "/Game/Blueprints/HUD/PickupPrompt.PickupPrompt_C"))
  (bind _output_get (Variables|Default|SetPickUpPromptRef _returnvalue))
  (UserInterface|Viewport|AddtoViewport _output_get 0)
  (Variables|Default|SetIsOverlappingItem true))

(event EventBeginPlay
  (Variables|Default|SetIsDead false)
  (bind _returnvalue (UserInterface|CreateWidget "/Game/Blueprints/HUD/HUD.HUD_C"))
  (bind _output_get (Variables|Default|SetHUD%20REFERENCE _returnvalue))
  (UserInterface|Viewport|AddtoViewport _output_get 0)
  (Input|SetInputModeGameOnly (Game|GetPlayerController 0))
  (bind _returnvalue_2 (SaveGame|LoadGamefromSlot "Slot1"))
  (bind _output_get_2 (Variables|Default|SetSaveGameInfo _returnvalue_2))
  (bind _assave_info (Utilities|Casting|CastToSaveInfo _output_get_2)
    (:then
      (Variables|Default|SetCurrency (Math|Float|Truncate (Variables|/Game/Blueprints/SaveInfo.SaveInfo_C|GetCurrency _assave_info))))
    (:CastFailed
      (Development|PrintString "Load Failed"))))

(event EventTick
  (params (DeltaSeconds :type Float%20%28single-precision%29))
  (Utilities|FlowControl|Sequence
    (:then_0
      (Utilities|SaveonDeath))
    (:then_1
      ;[1 1 1] EVENT TICK - IsCharging
      (if (Variables|Default|GetIsCharging)
        (Variables|Default|SetHeat (+ (Variables|Default|GetHeat) 0.01))
        (else
          (Variables|Default|SetHeat 0.0))))
    (:then_2
      (if (Variables|Default|GetIsZoomed)
        (Variables|Default|SetbUseControllerRotationYaw true)
        (else
          (Variables|Default|SetbUseControllerRotationYaw false))))))

(event Input|ActionEvents|InputActionPrimaryAim
  (params (Key :type Key%20Structure :default "AnyKey"))
  (:Pressed
    (Variables|Default|SetIsZoomed true)
    (Development|PrintString "ZoomIn"))
  (:Released
    (Variables|Default|SetIsZoomed false)
    (Development|PrintString "ZoomOut")))

(event Input|ActionEvents|InputActionPrimaryFire
  (params (Key :type Key%20Structure :default "AnyKey"))
  (:Pressed
    (Variables|Default|SetIsCharging true)
    (bind _newparam (CallFunction|Charging (Variables|Default|GetLeftHandArrow))))
  (:Released
    (CallFunction|PrimaryFire (Variables|Default|GetHeat))
    (Variables|Default|SetIsCharging false)
    (Components|DestroyComponent _newparam)
    (bind _returnvalue (Effects|SpawnEmitterAttached "/Game/Materials/ChargeBlast.ChargeBlast" (Variables|Default|GetLeftHandArrow) "None"))
    (Transformation|SetRelativeScale3D _returnvalue "0.100000,0.100000,0.100000")))

(event Input|ActionEvents|InputActionPause_TEMP
  (params (Key :type Key%20Structure :default "AnyKey"))
  (:Pressed
    (if (Variables|Default|GetIsPaused)
      (CallFunction|CloseMenu)
      (else
        (CallFunction|OpenMenu)))))

(event Input|ActionEvents|InputActionJump/Item
  (params (Key :type Key%20Structure :default "AnyKey"))
  (:Pressed
    (if (Variables|Default|GetIsOverlappingItem)
      (bind _asbasicitem (Utilities|Casting|CastToBasicitem (Utilities|Array|Get(acopy) (Collision|GetOverlappingActors "/Game/Blueprints/Basicitem.Basicitem_C" :!class /Script/Engine.Actor)))
        (:then
          (Variables|/Game/Blueprints/Basicitem.Basicitem_C|SetIsPickedUp _asbasicitem true))
        (:CastFailed
          (Development|PrintString "Hello")))
      (else
        (Character|Jump)))))

(event Input|ActionEvents|InputActionWeaponSwitch
  (params (Key :type Key%20Structure :default "AnyKey"))
  (:Pressed
    (if (== (Utilities|Array|Length (Variables|Default|GetWeaponArray)) (Variables|Default|GetCurrentWeaponInt))
      (Variables|Default|SetCurrentWeaponInt 0)
      (else
        (Variables|Default|SetCurrentWeaponInt (+ (Variables|Default|GetCurrentWeaponInt) 1))))))

(event Input|AxisEvents|InputAxisX_Camera
  (params (AxisValue :type Float%20%28single-precision%29))
  ;[1 1 1] Camera //TODO add controller vs mouse
  (Pawn|Input|AddControllerYawInput AxisValue))

(event Input|AxisEvents|InputAxisFwdMoveAxis
  (params (AxisValue :type Float%20%28single-precision%29))
  ;[1 1 1] Movement
  (Pawn|Input|AddMovementInput (Math|Vector|GetForwardVector (Math|Rotator|MakeRotator 0.0 0.0 (.Yaw (Math|Rotator|BreakRotator (Pawn|GetControlRotation :!class /Script/Engine.Pawn))))) AxisValue false))

(event Input|AxisEvents|InputAxisSideMoveAxis
  (params (AxisValue :type Float%20%28single-precision%29))
  ;[1 1 1] Movement
  (Pawn|Input|AddMovementInput (Math|Vector|GetRightVector (Math|Rotator|MakeRotator 0.0 0.0 (.Yaw (Math|Rotator|BreakRotator (Pawn|GetControlRotation :!class /Script/Engine.Pawn))))) AxisValue false))

(event Input|AxisEvents|InputAxisY_Camera
  (params (AxisValue :type Float%20%28single-precision%29))
  ;[1 1 1] Camera //TODO add controller vs mouse
  (Pawn|Input|AddControllerPitchInput AxisValue))

(fn ConstructionScript)

(fn PrimaryFire
  (params (ChargePercent :type Float%20%28single-precision%29))
  (bind _returnvalue (Pawn|GetControlRotation :!class /Script/Engine.Pawn))
  (bind (_roll _pitch) (Math|Rotator|BreakRotator _returnvalue))
  (if (<= ChargePercent 0.25)
    (Game|SpawnActorfromClass "/Game/Blueprints/EnergyBlast.EnergyBlast_C" (Math|Transform|MakeTransform (Transformation|GetWorldLocation (Variables|Default|GetLeftHandArrow)) (Math|Rotator|MakeRotator _roll _pitch (.Yaw (Math|Rotator|BreakRotator (Transformation|GetActorRotation)))) "1.000000,1.000000,1.000000") "AlwaysSpawn" 0 0.25 0)))

(fn Charging
  (params (TargetActor :type Scene%20Component%20Object%20Reference))
  (bind _returnvalue (Effects|SpawnEmitterAttached "/Game/Materials/Charge.Charge" TargetActor "None"))
  (Transformation|SetRelativeScale3D _returnvalue "0.400000,0.400000,0.400000")
  (return _returnvalue))

(fn OpenMenu
  (bind _returnvalue (UserInterface|CreateWidget "/Game/Blueprints/HUD/PauseMenu.PauseMenu_C"))
  (bind _output_get (Variables|Default|SetPauseMenuRef _returnvalue))
  (UserInterface|Viewport|AddtoViewport _output_get 0)
  (Variables|Default|SetIsPaused true)
  (Development|PrintString "true"))

(fn CloseMenu
  (Default|DestroyPause (Variables|Default|GetPauseMenuRef))
  (bind _output_get (Variables|Default|SetIsPaused false))
  (Development|PrintString (Utilities|String|ToString(Boolean) _output_get)))

(fn ShoulderZoomFunction
  (params (CurrentState :type Boolean) (BlendTrack :type Float%20%28single-precision%29)))

(fn PickupItem)