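; BasicGear_BrokenDontUse is a gear pickup actor, marked broken and not for use by its name.
; Overlap events show the pickup prompt on Player1_BP, then destroy it and clear IsOverlappingItem on exit.
; Tick polls IsPickedUp, which nothing here sets, then adds GearStats to the first player's GearTable and destroys the actor.
; The PickedUp event is an empty stub.
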(event Custom|PickedUp)

(event EventBeginPlay)

(event Collision|EventActorBeginOverlap
  (params (OtherActor :type Actor%20Object%20Reference))
  (bind _asplayer_1_bp (Utilities|Casting|CastToPlayer1_BP OtherActor))
  (Default|PickupPrompt _asplayer_1_bp))

(event EventTick
  (params (DeltaSeconds :type Float%20%28single-precision%29))
  (if (Variables|Default|GetIsPickedUp)
    (bind _asplayer_1_bp (Utilities|Casting|CastToPlayer1_BP (Game|GetPlayerCharacter 0)))
    (Utilities|Array|Add (Variables|/Game/Blueprints/Player1_BP.Player1_BP_C|GetGearTable _asplayer_1_bp) (Variables|Default|GetGearStats))
    (Actor|DestroyActor)))

(event Collision|EventActorEndOverlap
  (params (OtherActor :type Actor%20Object%20Reference))
  (bind _asplayer_1_bp (Utilities|Casting|CastToPlayer1_BP OtherActor))
  (Default|PickupPromptDestroy (Variables|/Game/Blueprints/Player1_BP.Player1_BP_C|GetPickUpPromptRef _asplayer_1_bp))
  (Variables|/Game/Blueprints/Player1_BP.Player1_BP_C|SetIsOverlappingItem _asplayer_1_bp false))

(fn ConstructionScript)