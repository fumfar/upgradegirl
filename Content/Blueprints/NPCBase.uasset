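; Base NPC actor that offers a talk prompt when the player overlaps it and shows dialogue line by line.
; Overlap adds the TalkWithNPCBase widget and sets IsTalking on Player1_BP.
; Each Talk call replaces the DialogueBase widget with the next FirstDialogue entry; the call after the last restores the prompt.
; Any end overlap clears both widgets and resets dialogue progress and talking flags, without checking which actor left.
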(event EventBeginPlay)

(event Collision|EventActorBeginOverlap
  (params (OtherActor :type Actor%20Object%20Reference))
  (if (not (Variables|Default|GetIsTalking))
    (CallFunction|TalkOptionOverlap OtherActor)))

(event EventTick
  (params (DeltaSeconds :type Float%20%28single-precision%29)))

(event Collision|EventActorEndOverlap
  (params (OtherActor :type Actor%20Object%20Reference))
  (Widget|RemovefromParent (Variables|Default|GetTalkOptionRef))
  (bind _asplayer_1_bp (Utilities|Casting|CastToPlayer1_BP (Game|GetPlayerCharacter 0)))
  (Variables|/Game/Blueprints/Player1_BP.Player1_BP_C|SetIsTalking _asplayer_1_bp false)
  (Variables|Default|SetFinishedTalking false)
  (Variables|Default|SetIsTalking false)
  (Widget|RemovefromParent (Variables|Default|GetCurrentDialogueRef))
  (Variables|Default|SetCurrentDialogueVar 0))

(fn ConstructionScript)

(fn TalkOptionOverlap
  (params (A :type Object%20Object%20Reference))
  (if (== A (Game|GetPlayerCharacter 0))
    (bind _returnvalue (UserInterface|CreateWidget "/Game/Blueprints/HUD/TalkWithNPCBase.TalkWithNPCBase_C" (Game|GetPlayerController 0)))
    (bind _output_get (Variables|Default|SetTalkOptionRef _returnvalue))
    (UserInterface|Viewport|AddtoViewport _output_get 0)
    (bind _asplayer_1_bp (Utilities|Casting|CastToPlayer1_BP (Game|GetPlayerCharacter 0)))
    (Variables|/Game/Blueprints/Player1_BP.Player1_BP_C|SetIsTalking _asplayer_1_bp true))
  (return))

(fn Talk
  (bind _firstdialogue (Variables|Default|GetFirstDialogue))
  (Utilities|SetIsTalkingtoTrue)
  (if (Variables|Default|GetFinishedTalking)
    (Widget|RemovefromParent (Variables|Default|GetCurrentDialogueRef))
    (Variables|Default|SetFinishedTalking false)
    (Variables|Default|SetIsTalking false)
    (bind _returnvalue (UserInterface|CreateWidget "/Game/Blueprints/HUD/TalkWithNPCBase.TalkWithNPCBase_C" (Game|GetPlayerController 0)))
    (bind _output_get (Variables|Default|SetTalkOptionRef _returnvalue))
    (UserInterface|Viewport|AddtoViewport _output_get 0)
    (else
      (if (> (Variables|Default|GetCurrentDialogueVar) 0)
        (Widget|RemovefromParent (Variables|Default|GetCurrentDialogueRef)))
      (bind _returnvalue_2 (UserInterface|CreateWidget "/Game/Blueprints/HUD/DialogueBase.DialogueBase_C"))
      (bind _output_get_2 (Variables|Default|SetCurrentDialogueRef _returnvalue_2))
      (UserInterface|Viewport|AddtoViewport _output_get_2 0)
      (bind _asdialogue_base (Utilities|Casting|CastToDialogueBase _returnvalue_2))
      (Variables|/Game/Blueprints/HUD/DialogueBase.DialogueBase_C|SetDialogueTextFromArray _asdialogue_base (Utilities|Array|Get(acopy) _firstdialogue (Variables|Default|GetCurrentDialogueVar)))
      (if (>= (Variables|Default|GetCurrentDialogueVar) (- (Utilities|Array|Length _firstdialogue) 1))
        (Variables|Default|SetIsTalking false)
        (Development|PrintString "Completed")
        (Variables|Default|SetCurrentDialogueVar 0)
        (Variables|Default|SetFinishedTalking true)
        (else
          (Variables|Default|SetCurrentDialogueVar (+ (Variables|Default|GetCurrentDialogueVar) 1)))))))