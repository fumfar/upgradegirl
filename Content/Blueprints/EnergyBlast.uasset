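; EnergyBlast is an energy projectile actor that deals damage and spawns an impact effect on hit.
; On Hit, SpawnEmitter1 applies energy-type damage, then spawns one of two emitters, chosen by the hit actor's "Enemy" tag and oriented to the surface normal.
; The blast then deactivates its own particle and destroys itself after a short delay.
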(event EventBeginPlay)

(event EventDestroyed)

(event Collision|EventHit
  (params (MyComp :type Primitive%20Component%20Object%20Reference) (Other :type Actor%20Object%20Reference) (OtherComp :type Primitive%20Component%20Object%20Reference) (bSelfMoved :type Boolean) (HitLocation :type Vector) (HitNormal :type Vector) (NormalImpulse :type Vector :default "0, 0, 0") (Hit :type Hit%20Result%20Structure%20%28by%20ref%29))
  (CallFunction|SpawnEmitter1 HitLocation (Math|Conversions|RotationFromXVector HitNormal) (.HitActor (Collision|BreakHitResult Hit)))
  (Components|Activation|Deactivate (Variables|Default|GetParticle1))
  (Utilities|FlowControl|Delay 5.0)
  (Actor|DestroyActor))

(fn ConstructionScript)

(fn SpawnEmitter1
  (params (HitLocation :type Vector) (HitRotation :type Rotator) (HitActor :type Actor%20Object%20Reference))
  (Game|Damage|ApplyDamage HitActor (Variables|Default|GetDamage) 0 0 "/Game/Blueprints/DamageTypeEnergy.DamageTypeEnergy_C")
  (if (Actor|ActorHasTag HitActor "Enemy")
    (Variables|Default|SetWhichEmitter "/Game/Materials/Emitters/BasicEmitter_2.BasicEmitter_2")
    (else
      (Variables|Default|SetWhichEmitter "/Game/Materials/Emitters/WallEmitter.WallEmitter")))
  (Effects|SpawnEmitteratLocation (Variables|Default|GetWhichEmitter) HitLocation HitRotation))